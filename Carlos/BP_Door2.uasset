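; BP_Door2 is a sliding door that opens automatically when the player character enters its Box trigger.
; Overlap plays the Open timeline, whose track scales a relative X offset on RightDoor while keeping Y and Z.
; On exit it waits one second, then reverses the timeline only if the InBox flag shows the player has not returned.
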(event `self.Box.OnComponentBeginOverlap`
  (params (OverlappedComponent :type "PrimitiveComponent Object Reference") (OtherActor :type "Actor Object Reference") (OtherComp :type "PrimitiveComponent Object Reference") (OtherBodyIndex :type Integer) (bFromSweep :type Boolean) (SweepResult :type "HitResult Structure (by ref)"))
  (bind _rightdoor (`self.RightDoor`))
  (bind (_relativelocation_x _relativelocation_y _relativelocation_z) (`KismetMathLibrary.BreakVector` (`SceneComponent.RelativeLocation` _rightdoor)))
  (cast `/Game/TPS_GameKit/BP_PlayerCharacter` OtherActor)
  (set `self.InBox` true)
  (bind (_direction _1) (`Timeline|Open` :`NewTime` 1.0 :!label _label)
    (:`Update`
      (`SceneComponent.K2_SetRelativeLocation` _rightdoor (`KismetMathLibrary.MakeVector` (* _1 120.0) _relativelocation_y _relativelocation_z) false false))))

(event `self.Box.OnComponentEndOverlap`
  (params (OverlappedComponent :type "PrimitiveComponent Object Reference") (OtherActor :type "Actor Object Reference") (OtherComp :type "PrimitiveComponent Object Reference") (OtherBodyIndex :type Integer))
  (cast `/Game/TPS_GameKit/BP_PlayerCharacter` OtherActor)
  (set `self.InBox` false)
  (`KismetSystemLibrary.Delay` 1.0)
  (if (not (`self.InBox`))
    (goto _label :!via `Reverse`)))

(fn `UserConstructionScript`)