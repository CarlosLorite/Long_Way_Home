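; Flower Blueprint for a collectible meant to be picked up by the player through a three-second left-mouse hold.
; Pressing sets a clicked flag after a delay, and releasing clears it without cancelling that delay.
; The flag is checked only when a Player-tagged actor begins overlapping; if set, the flower increments FlowersCollected and destroys itself.
; The counter is not yet linked to the player, as a comment notes the reference is pending.
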(event `Key|LeftMouseButton`
  (params (Key :type "Key Structure"))
  ;[1 1 1] Recoleccion de la flor (mantener pulsado por 3 segundos)
  (:`Pressed`
    (`KismetSystemLibrary.Delay` 3.0)
    (set `self.clickedButton` true))
  (:`Released`
    (set `self.clickedButton` false)))

(event `self.ReceiveActorBeginOverlap`
  (params (OtherActor :type "Actor Object Reference"))
  ;[1 1 1] Comprobacion del player
  (if (`self.ActorHasTag` OtherActor (`KismetStringLibrary.Conv_StringToName` (`self.player`)))
    (set `self.isNearFlower` true)
    (if (`self.isNearFlower`)
      ;[1 1 1] Eliminar flor
      (if (`self.clickedButton`)
        (`/Engine/EditorBlueprintResources/StandardMacros.IncrementInt` (`self.flowers_collected`)
          (:`  `
            (`self.K2_DestroyActor`)))))))

(event `self.ReceiveActorEndOverlap`
  (params (OtherActor :type "Actor Object Reference"))
  ;[1 1 1] Comprobacion del player
  (set `self.isNearFlower` false))

(fn `UserConstructionScript`)