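; Player Blueprint that prototypes a firearm with fire-rate control and magazine ammo.
; Left click, gated by cadence and ammo, spawns a timed-life actor at the pawn along control rotation, though no class is set and the impulse is zero.
; Each shot decrements and prints ammo, then waits out the cadence delay; Tick refreshes the ammo-available flag.
; A delayed reload with a full-magazine check exists but is never triggered.
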(event `Key|LeftMouseButton`
  (params (Key :type "Key Structure"))
  (bind _returnvalue (`GameplayStatics.GetPlayerPawn` 0))
  ;[1 1 1] Arma de Fuego
  ;;[1 1 1] Disparo Y Control de Cadencia
  ;;;[1 1 1] Intentar Disparar
  (:`Pressed`
    (if (`self.Cadencia Bool`)
      (if (`self.¿AmmoLeft?`)
        ;;;[1 1 1] Instanciar la Bala, dispararla y comenzar enfriamiento de la cadencia
        (bind _returnvalue_2 (`|SpawnActorFromClass` null (`KismetMathLibrary.MakeTransform` (`self.K2_GetActorLocation` _returnvalue) (`self.GetControlRotation` _returnvalue)) "Undefined" "OverrideRootScale" null null))
        (set `self.Cadencia Bool` false)
        (`PrimitiveComponent.AddImpulse` (* 0 (`self.GetActorForwardVector` _returnvalue_2)))
        ;;;[1 1 1] Eliminar bala con el tiempo
        (`self.SetLifeSpan` _returnvalue_2 (`self.InitialLifeSpan`))
        ;;;[1 1 1] Restar Bala del cargador
        (`/Engine/EditorBlueprintResources/StandardMacros.DecrementInt` (`self.AmmoLeft`)
          (:`  `
            ;;;[1 1 1] Control de Cadencia
            (`KismetSystemLibrary.Delay` (`self.Cadencia`))
            (set `self.Cadencia Bool` true)
            ;;;[1 1 1] Display ammo
            (`KismetSystemLibrary.PrintString` (`KismetStringLibrary.Conv_IntToString` (`self.AmmoLeft`)))))))))

(event `self.ReceiveTick`
  (params (DeltaSeconds :type "Float (single-precision)"))
  ;[1 1 1] Arma de Fuego
  ;;[1 1 1] Disparo Y Control de Cadencia
  ;;;[1 1 1] ¿Munición en el cargador?
  (`/Engine/EditorBlueprintResources/StandardMacros.CompareInt` (`self.AmmoLeft`)
    (:`>`
      (set `self.¿AmmoLeft?` true))
    (:`==`
      (set `self.¿AmmoLeft?` false :!label _label))
    (:`<`
      (goto _label))))

(fn `UserConstructionScript`)