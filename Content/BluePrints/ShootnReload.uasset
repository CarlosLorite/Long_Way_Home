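; Prototype firearm Blueprint for shooting, fire-rate control and reloading, driven by left mouse and a debug R key.
; A cadence flag and ammo check gate firing, while a custom event evaluates remaining ammo and R reports a full magazine.
; The shot itself (forward impulse, lifespan, ammo decrement), cooldown reset and magazine refill are disconnected, so input currently neither fires nor reloads.
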(event Custom|CustomEvent
  (params (DeltaSeconds :type Float%20%28single-precision%29))
  ;[1 1 1] Arma de Fuego
  ;;[1 1 1] Disparo Y Control de Cadencia
  ;;;[1 1 1] ¿Munición en el cargador?
  (Math|Integer|CompareInt (Variables|Default|GetAmmoLeft)
    (:>
      (Variables|Default|Set¿AmmoLeft? true))
    (:==
      (Variables|Default|Set¿AmmoLeft? false :!label _label))
    (:<
      (goto _label))))

(event Input|KeyboardEvents|DebugKeyR
  (params (Key :type Key%20Structure :default "None") (ActionValue :type Input%20Action%20Value%20Structure))
  ;[1 1 1] Arma de Fuego
  ;;[1 1 1] Recargar
  (:Pressed
    (Math|Integer|CompareInt (Variables|Default|GetAmmoLeft) (Variables|Default|GetMagazineCapacity)
      (:>
        _)
      (:==
        _))
    (Development|PrintString 0 "Cargador lleno")))

(event Input|MouseEvents|LeftMouseButton
  (params (Key :type Key%20Structure :default "None"))
  ;[1 1 1] Arma de Fuego
  ;;[1 1 1] Disparo Y Control de Cadencia
  ;;;[1 1 1] Intentar Disparar
  (:Pressed
    (if (Variables|Default|GetCadenciaBool)
      (if (Variables|Default|Get¿AmmoLeft?)
        _))))