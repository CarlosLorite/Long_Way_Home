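; BP_Wrek is an actor that handles proximity-based music around the player.
; BeginPlay starts music at the world origin.
; Each Tick compares the dot product of its forward vector and the direction to the player against AngleVision.
; When that value is below the threshold and the player is within a short distance, it plays tension music in 2D, with no guard against retriggering.
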(event `self.ReceiveBeginPlay`
  ;[1 1 1] musica
  (`GameplayStatics.PlaySoundAtLocation` null (0.0 0.0 0.0) (struct) 1.0 1.0 0.0 null null null null))

(event `self.ReceiveTick`
  (params (DeltaSeconds :type "Float (single-precision)"))
  (set `self.angle` (`KismetMathLibrary.Dot_VectorVector` (`KismetMathLibrary.Normal` (`self.GetActorForwardVector`)) (`KismetMathLibrary.Normal` (`self.DistPlayer`))))
  (bind _output_get (set `self.DistPlayer` (- (`self.K2_GetActorLocation` (`GameplayStatics.GetPlayerCharacter` 0)) (`self.K2_GetActorLocation`))))
  (if (and (<= (`KismetMathLibrary.VSize` _output_get) 20.0) (< (`self.angle`) (`self.AngleVision`)))
    ;[1 1 1] musica de tension
    (`GameplayStatics.PlaySound2D` null 1.0 1.0 0.0 null null)))

(fn `UserConstructionScript`)